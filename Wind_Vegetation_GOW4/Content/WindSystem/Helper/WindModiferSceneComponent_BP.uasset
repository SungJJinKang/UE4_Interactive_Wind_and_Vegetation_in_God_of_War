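; Scene component that acts as a wind modifier, writing its own velocity into wind map render targets.
; BeginPlay creates a dynamic instance of the modifier material; Tick is empty, so drawing relies on calls to DrawVelocityToTargetWindMaps.
; That function feeds component velocity and map origin into the material and draws it to the render target.
; It returns after the first valid target map, leaving any others untouched.
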(event EventBeginPlay
  (bind _returnvalue (Rendering|Material|CreateDynamicMaterialInstance (Variables|Default|GetWindModifierMaterial) "None" :!class /Script/Engine.KismetMaterialLibrary))
  (Variables|Default|SetWindModifierMaterialInstance _returnvalue))

(event EventTick
  (params (DeltaSeconds :type Float%20%28single-precision%29)))

(fn DrawVelocitytoTargetWindMaps
  (bind _windmodifiermaterialinstance (Variables|Default|GetWindModifierMaterialInstance))
  (for _array_element (Variables|Default|GetTargetWindMaps)
    (Utilities|IsValid _array_element
      (:Is%20Valid
        (Rendering|Material|SetVectorParameterValue _windmodifiermaterialinstance "WindVector" (Math|Conversions|ToLinearColor(Vector) (CallFunction|GetWindVector)) :!class /Script/Engine.MaterialInstanceDynamic)
        (Rendering|Material|SetVectorParameterValue _windmodifiermaterialinstance "WindMapOriginWorldPos" (Math|Conversions|ToLinearColor(Vector) (Variables|/Script/Wind_Vegetation_GOW4.WindMap|GetWindMapOriginWorldPosition _array_element)) :!class /Script/Engine.MaterialInstanceDynamic)
        (Rendering|DrawMaterialtoRenderTarget (Variables|/Script/Wind_Vegetation_GOW4.WindMap|GetWindMapRenderTarget2D _array_element) _windmodifiermaterialinstance)
        (return true)))))

(fn GetWindVector
  (return (Transformation|GetComponentVelocity)))
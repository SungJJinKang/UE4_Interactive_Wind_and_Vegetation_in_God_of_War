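; Base scene component for directional wind makers in the wind system, feeding directional wind parameters to a material.
; It extends the parent's material update by writing wind direction, range length and scale as material parameters.
; The direction comes from GetDirectionalWindVector, which returns a zero vector here and so adds no direction unless overridden.
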(event EventBeginPlay)

(event EventTick
  (params (DeltaSeconds :type Float%20%28single-precision%29))
  (|CallParentFunction DeltaSeconds))

(fn UpdateMaterialVariables
  (params (windMap :type Wind%20Map%20Object%20Reference) (material :type Material%20Instance%20Dynamic%20Object%20Reference))
  (|CallParentFunction windMap material)
  (Rendering|Material|SetVectorParameterValue material "WindDirection" (Math|Conversions|ToLinearColor(Vector) (CallFunction|GetDirectionalWindVector)) :!class /Script/Engine.MaterialInstanceDynamic)
  (Rendering|Material|SetScalarParameterValue material "WindRangeLength" (Variables|Default|GetWindRangeLength) :!class /Script/Engine.MaterialInstanceDynamic)
  (Rendering|Material|SetScalarParameterValue material "WindScale" (Variables|Default|GetWindScale) :!class /Script/Engine.MaterialInstanceDynamic))

(fn GetDirectionalWindVector
  (return "0.000000, 0, 0"))
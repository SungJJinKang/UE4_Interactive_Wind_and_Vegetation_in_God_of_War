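; Scene component for the wind system that acts as a directional wind motor driven by its own movement.
; Each tick, after the parent tick, it stores the change in its world location since the previous frame.
; GetDirectionalWindVector returns that raw delta as the wind vector, not normalized or divided by delta time, so its magnitude depends on frame rate.
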(event EventBeginPlay)

(event EventTick
  (params (DeltaSeconds :type Float%20%28single-precision%29))
  (|CallParentFunction DeltaSeconds)
  (CallFunction|UpdateDeltaWorldLocation))

(fn UpdateDeltaWorldLocation
  (bind _output_get (Variables|Default|SetPreviousWorldLocation (Variables|Default|GetCurrentWorldLocation)))
  (bind _output_get_2 (Variables|Default|SetCurrentWorldLocation (Transformation|GetWorldLocation)))
  (Variables|Default|SetDeltaWorldLocation (- _output_get_2 _output_get)))

(fn GetDirectionalWindVector
  (return (Variables|Default|GetDeltaWorldLocation)))
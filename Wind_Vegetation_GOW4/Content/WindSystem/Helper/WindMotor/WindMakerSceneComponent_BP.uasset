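; Wind motor scene component that adds its influence to wind maps, reporting its own component velocity as the wind vector.
; On BeginPlay it creates a dynamic instance of the wind modifier material.
; When passed a wind map in range, it updates that material with its origin and the map's default parameters.
; It then draws the material into the map's variance buffer render target, so the wind is written on the GPU.
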(event EventBeginPlay
  (|CallParentFunction)
  (CallFunction|CreateMaterialInstance))

(event EventTick
  (params (DeltaSeconds :type Float%20%28single-precision%29))
  (|CallParentFunction 0.0))

(event EventDrawWindVectortoPassedWindMap
  (params (windMap :type Wind%20Map%20Object%20Reference))
  (bind _returnvalue (Class|WindMap|GetVarianceBufferWindMapRenderTarget2D windMap))
  (bind _windmodifiermaterialinstancedynamic (Variables|Default|GetWindModifierMaterialInstanceDynamic))
  (Utilities|IsValid windMap
    (:Is%20Valid
      (Utilities|IsValid _returnvalue
        (:Is%20Valid
          (if (Class|WindModifierComponent|IsWindMapwithintheRangeOfWindModifier windMap)
            (CallFunction|UpdateMaterialVariables windMap _windmodifiermaterialinstancedynamic)
            (Rendering|DrawMaterialtoRenderTarget _returnvalue _windmodifiermaterialinstancedynamic)))))))

(fn GetWindVector
  (return (Transformation|GetComponentVelocity)))

(fn UpdateMaterialVariables
  (params (windMap :type Wind%20Map%20Object%20Reference) (material :type Material%20Instance%20Dynamic%20Object%20Reference))
  (Rendering|Material|SetVectorParameterValue material "OriginPos" (Math|Conversions|ToLinearColor(Vector) (Class|WindModifierComponent|GetModifierOriginLocation)) :!class /Script/Engine.MaterialInstanceDynamic)
  (CallFunction|SetWindMapDefaultMaterialParameters windMap))

(fn CreateMaterialInstance
  (bind _windmodifiermaterial (Variables|Default|GetWindModifierMaterial))
  (Utilities|IsValid _windmodifiermaterial
    (:Is%20Valid
      (bind _returnvalue (Rendering|Material|CreateDynamicMaterialInstance _windmodifiermaterial "None" :!class /Script/Engine.KismetMaterialLibrary))
      (Variables|Default|SetWindModifierMaterialInstanceDynamic _returnvalue))))
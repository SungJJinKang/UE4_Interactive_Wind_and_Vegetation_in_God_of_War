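; Wind modifier component that acts as a directional motor, pushing wind along the direction it moves.
; Each tick it stores its world location and computes the delta from the previous frame.
; When updating a wind map material, it passes the motor radius and that per-frame movement delta as the wind vector, on top of the parent modifier's parameters.
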(event EventBeginPlay)

(event EventTick
  (params (DeltaSeconds :type Float%20%28single-precision%29))
  (|CallParentFunction 0.0)
  (CallFunction|UpdateDeltaWorldLocation))

(fn UpdateDeltaWorldLocation
  (bind _output_get (Variables|Default|SetPreviousWorldLocation (Variables|Default|GetCurrentWorldLocation)))
  (bind _output_get_2 (Variables|Default|SetCurrentWorldLocation (Transformation|GetWorldLocation)))
  (Variables|Default|SetDeltaWorldLocation (- _output_get_2 _output_get)))

(fn UpdateMaterialVariables
  (params (windMap :type Wind%20Map%20Object%20Reference) (material :type Material%20Instance%20Dynamic%20Object%20Reference))
  (|CallParentFunction windMap material)
  (Rendering|Material|SetScalarParameterValue material "MotorRadius" (Variables|Default|GetMotorRadius) :!class /Script/Engine.MaterialInstanceDynamic)
  (Rendering|Material|SetVectorParameterValue material "WindVector" (Math|Conversions|ToLinearColor(Vector) (CallFunction|GetDirectionalWindVector)) :!class /Script/Engine.MaterialInstanceDynamic))

(fn GetDirectionalWindVector
  (return (Variables|Default|GetDeltaWorldLocation)))
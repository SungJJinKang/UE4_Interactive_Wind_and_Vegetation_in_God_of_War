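; Wind modifier component that paints a wind vector, by default its own component velocity, into wind map render targets.
; BeginPlay creates a dynamic instance of the modifier material.
; DrawVelocityToTargetWindMaps feeds it the wind vector, modifier origin and map transform basis, then draws it to the render target.
; The draw returns after the first valid target map, and nothing in this graph calls it.
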(event EventBeginPlay
  (|CallParentFunction)
  (CallFunction|CreateMaterialInstance))

(event EventTick
  (params (DeltaSeconds :type Float%20%28single-precision%29))
  (|CallParentFunction 0.0))

(fn DrawVelocitytoTargetWindMaps
  (bind _windmodifiermaterialinstancedynamic (Variables|Default|GetWindModifierMaterialInstanceDynamic))
  (CallFunction|UpdateWindVector)
  (bind _output_get (LocalVariables|SetTargetWindMapCount (Class|WindModifierComponent|GetTargetWindMapCount)))
  (for _index (range 0 _output_get)
    (bind (_outwindmap _returnvalue) (Class|WindModifierComponent|GetTargetWindMap _index))
    (if _returnvalue
      (CallFunction|UpdateMaterialVariables _outwindmap _windmodifiermaterialinstancedynamic)
      (Rendering|DrawMaterialtoRenderTarget (Variables|/Script/Wind_Vegetation_GOW4.WindMap|GetWindMapRenderTarget2D _outwindmap) _windmodifiermaterialinstancedynamic)
      (return true))))

(fn GetWindVector
  (return (Transformation|GetComponentVelocity)))

(fn UpdateWindMapTransfromMatrixBasis
  (params (windMap :type Wind%20Map%20Object%20Reference) (material :type Material%20Instance%20Dynamic%20Object%20Reference))
  (bind _windmaptransformmatrix (Variables|/Script/Wind_Vegetation_GOW4.WindMap|GetWindMapTransformMatrix windMap))
  (Rendering|Material|SetVectorParameterValue material "WindMapTransfromMatrixBasisX" (Math|Conversions|ToLinearColor(Vector) (Class|KismetMathLibrary|MatrixGetColumn _windmaptransformmatrix "First")) :!class /Script/Engine.MaterialInstanceDynamic)
  (Rendering|Material|SetVectorParameterValue material "WindMapTransfromMatrixBasisY" (Math|Conversions|ToLinearColor(Vector) (Class|KismetMathLibrary|MatrixGetColumn _windmaptransformmatrix "Second")) :!class /Script/Engine.MaterialInstanceDynamic)
  (Rendering|Material|SetVectorParameterValue material "WindMapTransfromMatrixBasisZ" (Math|Conversions|ToLinearColor(Vector) (Class|KismetMathLibrary|MatrixGetColumn _windmaptransformmatrix "Third")) :!class /Script/Engine.MaterialInstanceDynamic))

(fn UpdateWindVector
  (Rendering|Material|SetVectorParameterValue (Variables|Default|GetWindModifierMaterialInstanceDynamic) "WindVector" (Math|Conversions|ToLinearColor(Vector) (CallFunction|GetWindVector)) :!class /Script/Engine.MaterialInstanceDynamic))

(fn UpdateMaterialVariables
  (params (windMap :type Wind%20Map%20Object%20Reference) (material :type Material%20Instance%20Dynamic%20Object%20Reference))
  (CallFunction|UpdateWindMapTransfromMatrixBasis windMap material)
  (Rendering|Material|SetVectorParameterValue material "OriginPos" (Math|Conversions|ToLinearColor(Vector) (Class|WindModifierComponent|GetModifierOriginLocation)) :!class /Script/Engine.MaterialInstanceDynamic))

(fn CreateMaterialInstance
  (bind _windmodifiermaterial (Variables|Default|GetWindModifierMaterial))
  (Utilities|IsValid _windmodifiermaterial
    (:Is%20Valid
      (bind _returnvalue (Rendering|Material|CreateDynamicMaterialInstance _windmodifiermaterial "None" :!class /Script/Engine.KismetMaterialLibrary))
      (Variables|Default|SetWindModifierMaterialInstanceDynamic _returnvalue))))
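; Debug component that visualizes a wind map by drawing its wind vectors in the world.
; On BeginPlay it creates a cached float16 color wrapper, which DrawDebugTargetWindMap fills by reading back the map's front-buffer render target.
; The 2D texture is treated as depth slices stacked along its height, and each texel maps through the map's scale, offset, inverse rotation and origin to a world position.
; Toggles draw each RGB vector as an arrow or text.
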(event EventBeginPlay
  (|CallParentFunction)
  (bind _returnvalue (Game|ConstructObjectfromClass "/Script/Wind_Vegetation_GOW4.Float16ColorArrayWrapper" self))
  (Variables|Default|SetrenderTargetPixelFloat16ColorArrayWrapperCache _returnvalue))

(event EventTick
  (params (DeltaSeconds :type Float%20%28single-precision%29)))

(fn DrawDebugTargetWindMap
  (params (windMap :type Wind%20Map%20Object%20Reference))
  (bind _windmaprendertargetdepth (Variables|/Script/Wind_Vegetation_GOW4.WindMap|GetWindMapRenderTargetDepth windMap))
  (bind _rendertargetpixelfloat16colorarraywrappercache (Variables|Default|GetrenderTargetPixelFloat16ColorArrayWrapperCache))
  (|CallParentFunction windMap)
  (Utilities|IsValid windMap
    (:Is%20Valid
      (bind (_texturewidth _textureheight _returnvalue) (Class|RenderTarget2DHelper|ReadPixelsfromRenderTarget2D (Class|WindMap|GetFrontBufferWindMapRenderTarget2D windMap) (Variables|Default|GetrenderTargetPixelFloat16ColorArrayWrapperCache)))
      ;[1 1 1] Unit size of a wind
      (LocalVariables|SetunitSizeVec3 (/ (Variables|/Script/Wind_Vegetation_GOW4.WindMap|GetWindMapScaleInWorldSpace windMap) (Math|Vector|MakeVector (Math|Conversions|ToFloat(Integer) _texturewidth) (Math|Conversions|ToFloat(Integer) (/ _textureheight _windmaprendertargetdepth)) (Math|Conversions|ToFloat(Integer) _windmaprendertargetdepth))))
      (if _returnvalue
        ;[1 1 1] Iterate wind vector
        (for _index (range 0 (- _textureheight 1)) ; Y Loop
          (for _index_2 (range 0 (- _texturewidth 1)) ; X Loop
            ;[1 1 1] Pixel Index of texture
            (bind _output_get (LocalVariables|SetpixelIndex (+ (* (- (- _textureheight 1) _index) _texturewidth) (- (- _texturewidth 1) _index_2))))
            ;[1 1 1] Draw wind vector for debugging
            (if (Variables|Default|GetbTickDrawArrowsOfDebugTargetWindMaps)
              (Rendering|Debug|DrawDebugArrow (+ (Math|Conversions|ToVector(Vector4) (Class|KismetMathLibrary|MatrixTransformVector (Class|KismetMathLibrary|MatrixGetInverse (Variables|/Script/Wind_Vegetation_GOW4.WindMap|GetWindMapRotationMatrix windMap)) (+ (- (* (Variables|/Script/Wind_Vegetation_GOW4.WindMap|GetWindMapScaleInWorldSpace windMap) 0.5) (* (LocalVariables|GetunitSizeVec3) (Math|Vector|MakeVector (Math|Conversions|ToFloat(Integer) _index_2) (Math|Conversions|ToFloat(Integer) (Math|Integer|%(Integer) _index (/ _textureheight _windmaprendertargetdepth))) (Math|Conversions|ToFloat(Integer) (/ _index (/ _textureheight _windmaprendertargetdepth)))))) (Variables|/Script/Wind_Vegetation_GOW4.WindMap|GetWindMapOffsetInWorldSpace windMap)))) (Variables|/Script/Wind_Vegetation_GOW4.WindMap|GetWindMapOriginWorldPosition windMap)) (+ (* (Math|Vector|MakeVector (Class|Float16ColorArrayWrapper|R _rendertargetpixelfloat16colorarraywrappercache _output_get) (Class|Float16ColorArrayWrapper|G _rendertargetpixelfloat16colorarraywrappercache _output_get) (Class|Float16ColorArrayWrapper|B _rendertargetpixelfloat16colorarraywrappercache _output_get)) (Variables|Default|GetdebugDefaultArrowLengthScale)) (+ (Math|Conversions|ToVector(Vector4) (Class|KismetMathLibrary|MatrixTransformVector (Class|KismetMathLibrary|MatrixGetInverse (Variables|/Script/Wind_Vegetation_GOW4.WindMap|GetWindMapRotationMatrix windMap)) (+ (- (* (Variables|/Script/Wind_Vegetation_GOW4.WindMap|GetWindMapScaleInWorldSpace windMap) 0.5) (* (LocalVariables|GetunitSizeVec3) (Math|Vector|MakeVector (Math|Conversions|ToFloat(Integer) _index_2) (Math|Conversions|ToFloat(Integer) (Math|Integer|%(Integer) _index (/ _textureheight _windmaprendertargetdepth))) (Math|Conversions|ToFloat(Integer) (/ _index (/ _textureheight _windmaprendertargetdepth)))))) (Variables|/Script/Wind_Vegetation_GOW4.WindMap|GetWindMapOffsetInWorldSpace windMap)))) (Variables|/Script/Wind_Vegetation_GOW4.WindMap|GetWindMapOriginWorldPosition windMap))) (Variables|Default|GetdebugDefaultArrowSize) "(R=1.000000,G=1.000000,B=1.000000,A=1.000000)" 0.0 (Variables|Default|GetdebugDefaultArrowThickness)))
            (if (Variables|Default|GetbTickDrawWindVectorTextOfDebugTargetWindMaps)
              (Rendering|Debug|DrawDebugString (+ (Math|Conversions|ToVector(Vector4) (Class|KismetMathLibrary|MatrixTransformVector (Class|KismetMathLibrary|MatrixGetInverse (Variables|/Script/Wind_Vegetation_GOW4.WindMap|GetWindMapRotationMatrix windMap)) (+ (- (* (Variables|/Script/Wind_Vegetation_GOW4.WindMap|GetWindMapScaleInWorldSpace windMap) 0.5) (* (LocalVariables|GetunitSizeVec3) (Math|Vector|MakeVector (Math|Conversions|ToFloat(Integer) _index_2) (Math|Conversions|ToFloat(Integer) (Math|Integer|%(Integer) _index (/ _textureheight _windmaprendertargetdepth))) (Math|Conversions|ToFloat(Integer) (/ _index (/ _textureheight _windmaprendertargetdepth)))))) (Variables|/Script/Wind_Vegetation_GOW4.WindMap|GetWindMapOffsetInWorldSpace windMap)))) (Variables|/Script/Wind_Vegetation_GOW4.WindMap|GetWindMapOriginWorldPosition windMap)) (Utilities|String|ToString(Vector) (Math|Vector|MakeVector (Class|Float16ColorArrayWrapper|R _rendertargetpixelfloat16colorarraywrappercache _output_get) (Class|Float16ColorArrayWrapper|G _rendertargetpixelfloat16colorarraywrappercache _output_get) (Class|Float16ColorArrayWrapper|B _rendertargetpixelfloat16colorarraywrappercache _output_get))) 0 "(R=1.000000,G=1.000000,B=1.000000,A=1.000000)"))))))))
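; WindMap_BP is the Blueprint layer of the wind map system, feeding per-tick wind data to the materials that process the wind map.
; On initialization it creates a dynamic material instance from the default post-process material.
; Before each wind map tick, it writes the static wind vector to a material parameter collection and passes the variance render target, speed-to-static-wind vector and previous map origin to that instance.
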(event EventPreTickWindMap
  (bind _windmappostprocessmaterialinstance (Variables|Default|GetWindMapPostProcessMaterialInstance))
  (|CallParentFunction)
  (Utilities|IsValid _windmappostprocessmaterialinstance
    (:Is%20Valid
      (Rendering|Material|SetVectorParameterValue self "/Game/WindSystem/Helper/HelperMaterail/WindMapMaterialCollection.WindMapMaterialCollection" "StaticWindVector" (Math|Conversions|ToLinearColor(Vector) (Variables|Default|GetStaticWindVector)) :!class /Script/Engine.KismetMaterialLibrary)
      (Rendering|Material|SetTextureParameterValue _windmappostprocessmaterialinstance "WindMapVarianceBuffer" (Class|WindMap|GetVarianceBufferWindMapRenderTarget2D))
      (Rendering|Material|SetVectorParameterValue _windmappostprocessmaterialinstance "SpeedToStaticWindVector" (Math|Conversions|ToLinearColor(Vector) (Variables|Default|GetSpeedToStaticWindVector)) :!class /Script/Engine.MaterialInstanceDynamic)
      (Rendering|Material|SetVectorParameterValue _windmappostprocessmaterialinstance "PreviousTickWindMapOriginWorldPosition" (Math|Conversions|ToLinearColor(Vector) (Variables|Default|GetPreviousTickWindMapOriginWorldPosition)) :!class /Script/Engine.MaterialInstanceDynamic))))

(event EventPostTickWindMap
  (|CallParentFunction))

(event EventInitializeWindMap
  (bind _defaultpostprocessmaterial (Variables|Default|GetDefaultPostProcessMaterial))
  (Utilities|IsValid _defaultpostprocessmaterial
    (:Is%20Valid
      (bind _returnvalue (Rendering|Material|CreateDynamicMaterialInstance self _defaultpostprocessmaterial "None" :!class /Script/Engine.KismetMaterialLibrary))
      (Variables|Default|SetWindMapPostProcessMaterialInstance _returnvalue))))